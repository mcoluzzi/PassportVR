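; BP_Fluorite is a fluorite object that can be picked up and reveals a plane while it sits inside a CleavageBox.
; Begin and end overlap with CleavageBox set IsInBox, which Tick uses to show or hide the Plane component.
; Tick also restores query and physics collision on the mesh whenever it is disabled.
; Pickup stops physics and attaches the root to the given component, and Drop restores physics and detaches.
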(event `self.ReceiveTick`
  (params (DeltaSeconds :type "Float (single-precision)"))
  (bind _plane (`self.Plane`))
  (bind _staticmeshcomponent (`self.StaticMeshComponent`))
  (bind _plane_2 (`self.Plane`))
  (if (`|EnumEquality` (`PrimitiveComponent.GetCollisionEnabled` _staticmeshcomponent) "NoCollision")
    (`PrimitiveComponent.SetCollisionEnabled` _staticmeshcomponent "QueryAndPhysics"))
  (if (`self.isInBox`)
    (if (not (`SceneComponent.IsVisible` _plane))
      (`SceneComponent.SetVisibility` _plane true false))
    (elif (`SceneComponent.IsVisible` _plane_2)
      (`SceneComponent.SetVisibility` _plane_2 false false))))

(event `self.ReceiveActorBeginOverlap`
  (params (OtherActor :type "Actor Object Reference"))
  (if (== (`GameplayStatics.GetObjectClass` OtherActor) "/Game/VirtualRealityBP/Blueprints/CleavageBox.CleavageBox_C")
    (set `self.isInBox` true)))

(event `self.ReceiveActorEndOverlap`
  (params (OtherActor :type "Actor Object Reference"))
  (if (== (`GameplayStatics.GetObjectClass` OtherActor) "/Game/VirtualRealityBP/Blueprints/CleavageBox.CleavageBox_C")
    (set `self.isInBox` false)))

(event `/Game/VirtualRealityBP/Blueprints/PickupActorInterface.Pickup`
  (params (AttachTo :type "SceneComponent Object Reference"))
  (`PrimitiveComponent.SetSimulatePhysics` (`self.StaticMeshComponent`) false)
  (`SceneComponent.K2_AttachToComponent` (`self.K2_GetRootComponent`) AttachTo "None" "KeepWorld" "KeepWorld" "KeepWorld" false))

(event `/Game/VirtualRealityBP/Blueprints/PickupActorInterface.Drop`
  (`PrimitiveComponent.SetSimulatePhysics` (`self.StaticMeshComponent`) true)
  (`self.K2_DetachFromActor` "KeepWorld" "KeepWorld" "KeepWorld"))

(fn `UserConstructionScript`)